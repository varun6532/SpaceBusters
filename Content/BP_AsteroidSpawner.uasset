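; Actor that continuously spawns BP_Asteroid obstacles ahead of the player's ship.
; A looping 0.1-second timer started on BeginPlay runs the spawn event, which only proceeds if the player pawn is a BP_PlayerShip.
; Each asteroid appears a fixed distance along world +X from the ship, with random Y and Z offsets, using the spawner's own rotation.
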(event `self.ReceiveBeginPlay`
  (`KismetSystemLibrary.K2_SetTimerDelegate` (delegate `Spawner`) 0.1 true))

(event `Spawner`
  (bind _asbp_player_ship (cast `/Game/BP_PlayerShip` (`GameplayStatics.GetPlayerPawn` 0)))
  (bind (_returnvalue_x _returnvalue_y _returnvalue_z) (`KismetMathLibrary.BreakVector` (`self.K2_GetActorLocation` _asbp_player_ship)))
  (`|SpawnActorFromClass` "/Game/BP_Asteroid.BP_Asteroid_C" (`KismetMathLibrary.MakeTransform` (`KismetMathLibrary.MakeVector` (+ _returnvalue_x 4000.0) (+ (`KismetMathLibrary.RandomFloatInRange` -2000.0 2000.0) _returnvalue_y) (+ (`KismetMathLibrary.RandomFloatInRange` -400.0 400.0) _returnvalue_z)) (`self.K2_GetActorRotation`)) "Undefined" "MultiplyWithRoot" null null))

(fn `UserConstructionScript`)