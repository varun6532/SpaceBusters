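; Player-controlled spaceship that dodges and shoots at asteroids, creating the score HUD when play begins.
; Move and Steering axes offset the ship vertically and sideways, while right mouse fires projectiles from two arrow components with a laser sound.
; Four collision components set Finishedgame on asteroid overlap.
; Tick polls that flag to swap the HUD for a game-over widget, blend to the tagged post-game camera, show the cursor and pause.
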(event `self.ReceiveBeginPlay`
  (bind _returnvalue (`|CreateWidget` "/Game/WB_Score.WB_Score_C"))
  (`UserWidget.AddToViewport` _returnvalue 0))

(event `self.ReceiveTick`
  (params (DeltaSeconds :type "Float (single-precision)"))
  (if (`self.Finishedgame`)
    (`Widget.RemoveFromParent` (stale `self.ReceiveBeginPlay` _returnvalue))
    (bind _outactors (`GameplayStatics.GetAllActorsOfClassWithTag` "/Script/CinematicCamera.CineCameraActor" "PostGameCamera"))
    (`PlayerController.SetViewTargetWithBlend` (`GameplayStatics.GetPlayerController` 0) (`|GetArrayItem` _outactors) 0.0 "VTBlend_Linear" 0.0 false)
    (bind _returnvalue (`|CreateWidget` "/Game/WB_GameOver.WB_GameOver_C"))
    (`UserWidget.AddToViewport` _returnvalue 0)
    (set `PlayerController.bShowMouseCursor` true (`GameplayStatics.GetPlayerController` 0))
    (`GameplayStatics.SetGamePaused` true)))

(event `Key|Escape`
  (params (Key :type "Key Structure"))
  (:`Pressed`
    (`KismetSystemLibrary.PrintString` "No pause menu here lil bro")))

(event `InputAxis|Move`
  (params (AxisValue :type "Float (single-precision)"))
  (`self.K2_AddActorLocalOffset` (`KismetMathLibrary.MakeVector` 0.0 0.0 (* AxisValue (`self.SideSpeed_0`) (stale `self.ReceiveTick` DeltaSeconds)))))

(event `InputAxis|Steering`
  (params (AxisValue :type "Float (single-precision)"))
  (`self.K2_AddActorLocalOffset` (`KismetMathLibrary.MakeVector` 0.0 (* (`self.SideSpeed_0`) AxisValue (stale `self.ReceiveTick` DeltaSeconds)))))

(event `Key|RightMouseButton`
  (params (Key :type "Key Structure"))
  (:`Pressed`
    (`|SpawnActorFromClass` "/Game/BP_Projectile.BP_Projectile_C" (`SceneComponent.K2_GetComponentToWorld` (`self.ProjectileArrowRight`)) "Undefined" "MultiplyWithRoot" null null)
    (`|SpawnActorFromClass` "/Game/BP_Projectile.BP_Projectile_C" (`SceneComponent.K2_GetComponentToWorld` (`self.ProjectileArrowLeft`)) "Undefined" "MultiplyWithRoot" null null)
    (`GameplayStatics.SpawnSound2D` "/Game/Assets/Lights/lasersfx.lasersfx" 1.0 1.0 0.0 null)))

(event `self.Box1.OnComponentBeginOverlap`
  (params (OverlappedComponent :type "PrimitiveComponent Object Reference") (OtherActor :type "Actor Object Reference") (OtherComp :type "PrimitiveComponent Object Reference") (OtherBodyIndex :type Integer) (bFromSweep :type Boolean) (SweepResult :type "HitResult Structure (by ref)"))
  (cast `/Game/BP_Asteroid` OtherActor)
  (set `self.Finishedgame` true))

(event `self.Box.OnComponentBeginOverlap`
  (params (OverlappedComponent :type "PrimitiveComponent Object Reference") (OtherActor :type "Actor Object Reference") (OtherComp :type "PrimitiveComponent Object Reference") (OtherBodyIndex :type Integer) (bFromSweep :type Boolean) (SweepResult :type "HitResult Structure (by ref)"))
  (cast `/Game/BP_Asteroid` OtherActor)
  (set `self.Finishedgame` true))

(event `self.w.OnComponentBeginOverlap`
  (params (OverlappedComponent :type "PrimitiveComponent Object Reference") (OtherActor :type "Actor Object Reference") (OtherComp :type "PrimitiveComponent Object Reference") (OtherBodyIndex :type Integer) (bFromSweep :type Boolean) (SweepResult :type "HitResult Structure (by ref)"))
  (cast `/Game/BP_Asteroid` OtherActor)
  (set `self.Finishedgame` true))

(event `self.w1.OnComponentBeginOverlap`
  (params (OverlappedComponent :type "PrimitiveComponent Object Reference") (OtherActor :type "Actor Object Reference") (OtherComp :type "PrimitiveComponent Object Reference") (OtherBodyIndex :type Integer) (bFromSweep :type Boolean) (SweepResult :type "HitResult Structure (by ref)"))
  (cast `/Game/BP_Asteroid` OtherActor)
  (set `self.Finishedgame` true))

(fn `UserConstructionScript`)